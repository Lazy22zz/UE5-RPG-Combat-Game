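; Base enemy character Blueprint that handles the dissolve-in entrance and the death sequence of Warrior enemies.
; BeginPlay runs a reversed dissolve timeline on the mesh and equipped weapon materials while playing a random entry montage.
; On death it pauses animation, disables capsule collision, removes enemy widgets and attaches an async-loaded Niagara effect tinted by the material's edge color.
; When the death dissolve finishes, it destroys the weapon, tries the SpawnStones ability, then destroys itself.
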(event EventBeginPlay
  (bind _entryanim_montage (Variables|Default|GetEntryAnim%20Montage))
  (bind _enemycombatcomponent (Variables|Default|GetEnemyCombatComponent))
  (bind _returnvalue (Class|PawnCombatComponent|GetCharacterCurrentEquippedWeapon _enemycombatcomponent))
  (Utilities|FlowControl|Sequence
    (:then_0
      (Components|Timeline|SetPlayRate (Variables|Default|GetEntryDisolveTimeline) (/ 1.0 (Variables|Default|GetTotal%20Entry%20Time%20Rate)))
      (bind _normalizefloattrack (Timeline|EntryDisolveTimeline ReverseFromEnd)
        (:Update
          (Rendering|Material|SetScalarParameterValueonMaterials (Variables|Character|GetMesh) "DissolveAmount" _normalizefloattrack)
          (Utilities|IsValid _returnvalue
            (:Is%20Valid
              (Rendering|Material|SetScalarParameterValueonMaterials (Variables|/Script/Warrior.WarriorWeaponBase|GetWeaponMesh _returnvalue) "DissolveAmount" _normalizefloattrack))))))
    (:then_1
      (if (Utilities|Array|IsNotEmpty _entryanim_montage)
        (Animation|PlayAnimMontage (.OutItem (Utilities|Array|Random _entryanim_montage)) 1.0 "None")))))

(event EventOnenemyDied
  (params (DissolveNiagaraSystem :type Niagara%20System%20Soft%20Object%20Reference))
  (bind _enemycombatcomponent (Variables|Default|GetEnemyCombatComponent))
  (bind _enemycombatcomponent_2 (Variables|Default|GetEnemyCombatComponent))
  (bind _mesh (Variables|Character|GetMesh))
  (bind _returnvalue (Class|PawnCombatComponent|GetCharacterCurrentEquippedWeapon _enemycombatcomponent))
  (bind _returnvalue_2 (Class|PawnCombatComponent|GetCharacterCurrentEquippedWeapon _enemycombatcomponent_2))
  (Utilities|FlowControl|Sequence
    (:then_0
      ;[1 1 1] Disable collision
      (Variables|/Script/Engine.SkeletalMeshComponent|SetbPauseAnims (Variables|Character|GetMesh) true)
      (Collision|SetCollisionEnabled (Variables|Default|GetCapsuleComponent) "NoCollision"))
    (:then_1
      ;[1 1 1] Remove UI
      (Class|EnemyUIComponent|RemoveAnyEnemyWidgetsifAny (Variables|Default|GetEnemyUIComponent)))
    (:then_2
      (bind _object (Utilities|AsyncLoadAsset DissolveNiagaraSystem)
        (:then
          _)
        (:Completed
          _))
      (bind _asniagara_system (Utilities|Casting|CastToNiagaraSystem _object))
      (bind _returnvalue_3 (Niagara|SpawnSystemAttached _asniagara_system (Variables|Character|GetMesh) "None" "0, 0, 0" "0, 0, 0" "KeepRelativeOffset" true))
      (bind _returnvalue_4 (Rendering|Material|CreateDynamicMaterialInstance _mesh 0 (Rendering|Material|GetMaterial _mesh 0) "None" :!class /Script/Engine.PrimitiveComponent))
      (bind _returnvalue_5 (Rendering|Material|GetVectorParameterValue _returnvalue_4 "DissolveEdgeColor" :!class /Script/Engine.MaterialInstanceDynamic))
      (Niagara|SetNiagaraVariable(LinearColor) _returnvalue_3 "DissolveParticleColor" _returnvalue_5)
      (Components|Timeline|SetPlayRate (Variables|Default|GetDissolveTimeline) (/ 1.0 (Variables|Default|GetTotalDissolveTime)))
      (bind _normalizefloattrack (Timeline|DissolveTimeline PlayFromStart)
        (:Update
          (Rendering|Material|SetScalarParameterValueonMaterials (Variables|Character|GetMesh) "DissolveAmount" _normalizefloattrack)
          (Utilities|IsValid _returnvalue
            (:Is%20Valid
              (Rendering|Material|SetScalarParameterValueonMaterials (Variables|/Script/Warrior.WarriorWeaponBase|GetWeaponMesh _returnvalue) "DissolveAmount" _normalizefloattrack))))
        (:Finished
          (Utilities|IsValid _returnvalue_2
            (:Is%20Valid
              (Actor|DestroyActor _returnvalue_2))
            (:Is%20Not%20Valid
              _))
          (Class|WarriorAbilitySystemComponent|TryActivateAbilitybyTag (Variables|Default|GetWarriorAbilitySystemComponent) "(TagName=\"Enemy.Ability.SpawnStones\")")
          (Utilities|FlowControl|Delay 0.5)
          (Actor|DestroyActor))))))

(fn ConstructionScript)