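; Base enemy gameplay ability that may drop a healing or rage stone near the enemy.
; It traces down to the ground and picks a random navigable point around the hit.
; A level-scaled curve sets the drop chance, and an even coin flip picks the stone type.
; The class loads asynchronously before spawning, with a random angle-sized value wired into Z scale rather than rotation.
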(event Ability|EventActivateAbility
  (bind _returnvalue (Class|WarriorEnemyGameplayAbility|GetEnemyCharacterfromActorInfo))
  (bind _returnvalue_2 (Transformation|GetActorLocation _returnvalue))
  (Utilities|FlowControl|Sequence
    (:then_0
      ;[1 1 1] Spawn Random Stones At Hit Line Trace Location
      (bind _outhit (Collision|LineTraceForObjects _returnvalue_2 (+ _returnvalue_2 (* (Transformation|GetActorUpVector _returnvalue) -2e+02)) (Variables|Default|GetObject%20Types) false 0 "None"))
      (bind _randomlocation (Class|NavigationSystemV1|GetRandomLocationinNavigableRadius (.ImpactPoint (Collision|BreakHitResult _outhit)) 2e+02 0 0))
      (Variables|Default|SetRandomSpawnStoneLocation _randomlocation))
    (:then_1
      ;[1 1 1] Async Load Class
      (if (Math|Random|RandomBoolwithWeight 0.5)
        (Variables|Default|SetAsset%20Class "/Game/Items/Stones/BP_HealingStones.BP_HealingStones_C")
        (else
          (Variables|Default|SetAsset%20Class "/Game/Items/Stones/BP_RageStones.BP_RageStones_C")))
      (if (Math|Random|RandomBoolwithWeight (Class|WarriorFunctionLibrary|GetScalableFloatValueatLevel (Variables|Default|GetSpawnStoneScaledFloat) (Math|Conversions|ToFloat(Integer) (Ability|GetAbilityLevel))))
        (bind _class (Utilities|AsyncLoadClassAsset (Variables|Default|GetAsset%20Class))
          (:Completed
            (bind _asactor (Utilities|Casting|CastToActorClass _class)
              (:then
                ;[1 1 1] Spawn cast Async class to actor location
                (Game|SpawnActorfromClass _asactor (Math|Transform|MakeTransform (Variables|Default|GetRandomSpawnStoneLocation) "0, 0, 0" (Math|Vector|MakeVector 1.0 1.0 (Math|Random|RandomFloatinRange 0.0 3.6e+02))) "AdjustIfPossibleButAlwaysSpawn" "MultiplyWithRoot" 0 0)
                (Ability|EndAbility))
              (:CastFailed
                (Ability|EndAbility)))))
        (else
          (Ability|EndAbility))))))

(event Ability|EventOnEndAbility
  (params (bWasCancelled :type Boolean)))