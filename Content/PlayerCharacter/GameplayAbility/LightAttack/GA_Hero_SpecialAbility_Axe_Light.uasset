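; Hero gameplay ability for the axe's light special attack, which plays a montage and ends when it completes, blends out or is interrupted or cancelled.
; On start it commits the ability and notifies the hero UI of the cooldown.
; Melee hit events apply light-attack damage from the equipped weapon's damage at ability level, using a fixed combo count.
; Successful hits trigger an axe sound cue and send a hit react event to the target.
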(event Ability|EventActivateAbility
  (bind _returnvalue (Class|GameplayAbility|GetCooldownTimeRemaining))
  (|PlayMontageandWaitProxy "None" "/Game/PlayerCharacter/Montages/AM_Hero_Axe_Ability_Light.AM_Hero_Axe_Ability_Light" 1.0 "None" true 1.0 0.0 false
    (:then
      (Utilities|FlowControl|Sequence
        (:then_0
          (bind _payload (Ability|Tasks|WaitGameplayEvent "(TagName=\"Shared.Event.MeleeHit\")" 0)
            (:EventReceived
              (CallFunction|HandleApplyDamage _payload))))
        (:then_1
          ;[1 1 1] Special Ability Cooldown UI
          (Ability|CommitAbility)
          (Default|CallOnAbilityCooldownBeginDelegate (Variables|/Script/Warrior.WarriorHeroCharacter|GetHeroUIComponent (Class|WarriorHeroGameplayAbility|GetHeroCharacterfromActorInfo)) "(TagName=\"InputTag.SpecialWeaponAbility.Light\")" _returnvalue _returnvalue))))
    (:OnCompleted
      (Ability|EndAbility :!label _label))
    (:OnBlendOut
      (goto _label))
    (:OnInterrupted
      (goto _label))
    (:OnCancelled
      (goto _label))))

(event Ability|EventOnEndAbility
  (params (bWasCancelled :type Boolean)))

(fn HandleApplyDamage
  (params (InPayLoad :type Gameplay%20Event%20Data%20Structure))
  ;[1 1 1] Apply Damage Base on Weapon damage on level
  (bind _output_get (LocalVariables|SetGetHitTarget (.Target (Utilities|Struct|BreakGameplayEventData InPayLoad))))
  (Class|WarriorGameplayAbility|ApplyEffectSpecHandletoTarget _output_get (Class|WarriorHeroGameplayAbility|MakeHeroDamageEffectSpecHandle "/Game/Shared/GameplayEffect/GE_Shared_DealDamage.GE_Shared_DealDamage_C" (Class|HeroCombatComponent|GetHeroCurrentEquippWeaponDamageatLevel (Class|WarriorHeroGameplayAbility|GetHeroCombatComponentfromActorInfo) (Math|Conversions|ToFloat(Integer) (Ability|GetAbilityLevel))) "(TagName=\"Player.SetByCaller.AttackType.Light\")" 4)
    (:Successful
      ;[1 1 1] Play Hit Sound
      (GameplayCue|ExecuteGameplayCue :GameplayCueTag "(TagName=\"GameplayCue.Sounds.MeleeHit.AxeHit\")")
      ;[1 1 1] Send Hit React to enemy
      (Ability|SendGameplayEventtoActor (LocalVariables|GetGetHitTarget) "(TagName=\"Shared.Ability.HitReact\")" InPayLoad))))